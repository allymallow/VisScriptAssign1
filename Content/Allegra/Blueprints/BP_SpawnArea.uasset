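; BP_SpawnArea is a placeable volume that scatters BP_Collectable actors inside its box when play begins.
; On BeginPlay it spawns NumberOfSpawns collectables at random points within the SpawnExtent box, each with zero rotation and unit scale, and stores them in CollectableArray.
; Spawns adjust to avoid collisions and are skipped if no free spot is found, and the final array length is logged.
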(event `self.ReceiveBeginPlay`
  (for _ (range 1 (+ (`self.NumberOfSpawns`) 1))
    (bind _returnvalue (`|SpawnActorFromClass` "/Game/Allegra/Blueprints/BP_Collectable.BP_Collectable_C" (`self.GetRandomLocationInSpawn`) "AdjustIfPossibleButDontSpawnIfColliding" "MultiplyWithRoot" null null))
    (`KismetArrayLibrary.Array_Add` (`self.CollectableArray`) _returnvalue))
  (`KismetSystemLibrary.PrintString` (`KismetStringLibrary.Concat_StrStr` "ArrayLength" (`KismetStringLibrary.Conv_IntToString` (`KismetArrayLibrary.Array_Length` (`self.CollectableArray`)))) false))

(fn `GetRandomLocationInSpawn`
  (returns (RandomLocation :type "Transform Structure"))
  (bind _spawnextent (`self.SpawnExtent`))
  (return (`KismetMathLibrary.MakeTransform` (`KismetMathLibrary.RandomPointInBoundingBox` (`SceneComponent.K2_GetComponentLocation` _spawnextent) (`BoxComponent.BoxExtent` _spawnextent)))))

(fn `UserConstructionScript`)